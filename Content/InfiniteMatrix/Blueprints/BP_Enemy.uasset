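; BP_Enemy is an enemy actor that damages the player on contact and is destroyed by projectiles.
; A Sphere overlap runs two cast checks: touching BP_Player lowers health, refreshes the health UI and plays a thud.
; A BP_Projectile hit calls score and score UI updates on player pawn 0, plays a spark sound and destroys the enemy.
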(event `self.Sphere.OnComponentBeginOverlap`
  (params (OverlappedComponent :type "PrimitiveComponent Object Reference") (OtherActor :type "Actor Object Reference") (OtherComp :type "PrimitiveComponent Object Reference") (OtherBodyIndex :type Integer) (bFromSweep :type Boolean) (SweepResult :type "HitResult Structure (by ref)"))
  (`|ExecutionSequence`
    (:`then_0`
      (bind _asbp_player (cast `/Game/InfiniteMatrix/Blueprints/BP_Player` OtherActor))
      (`/Game/InfiniteMatrix/Blueprints/BP_Player.HealthDown` _asbp_player)
      (`/Game/InfiniteMatrix/Blueprints/BP_Player.UpdateHealthUI` _asbp_player)
      (`GameplayStatics.PlaySoundAtLocation` "/Game/InfiniteMatrix/Audio/thud-291047.thud-291047" (`SceneComponent.K2_GetComponentLocation` (`self.StaticMesh`)) (struct) 1.0 1.0 0.0 null null null null))
    (:`then_1`
      (cast `/Game/InfiniteMatrix/Blueprints/BP_Projectile` OtherActor)
      (bind _asbp_player_2 (cast `/Game/InfiniteMatrix/Blueprints/BP_Player` (`GameplayStatics.GetPlayerPawn` 0)))
      (`/Game/InfiniteMatrix/Blueprints/BP_Player.ScoreUp` _asbp_player_2)
      (`/Game/InfiniteMatrix/Blueprints/BP_Player.UpdateScoreUI` _asbp_player_2)
      (`GameplayStatics.PlaySoundAtLocation` "/Game/InfiniteMatrix/Audio/electronic-element-burn-spark-1-248606.electronic-element-burn-spark-1-248606" (`SceneComponent.GetSocketLocation` (`self.StaticMesh`) "None") (struct) 1.0 1.0 0.0 null null null null)
      (`self.K2_DestroyActor`))))

(fn `UserConstructionScript`)