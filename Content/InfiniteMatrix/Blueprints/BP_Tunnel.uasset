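; BP_Tunnel is a tunnel segment for an endless obstacle game, with a rotating wall that takes a random hole mesh and roll through RandomizeWall.
; Hitting the wall costs a living player health and score, showing restart at zero health.
; The exit trigger awards score, with a sound on clean passes, requests the next tunnel and destroys this one; it also destroys projectiles.
; SpawnHealth and SpawnEnemy randomly place short-lived pickups and enemies inside box zones.
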(event `self.ReceiveTick`
  (params (DeltaSeconds :type "Float (single-precision)"))
  (`SceneComponent.K2_AddLocalRotation` (`self.WallMesh`) (`KismetMathLibrary.MakeRotator` (* DeltaSeconds (`self.RotateSpeed`))) false false))

(event `self.TriggerZone.OnComponentBeginOverlap`
  (params (OverlappedComponent :type "PrimitiveComponent Object Reference") (OtherActor :type "Actor Object Reference") (OtherComp :type "PrimitiveComponent Object Reference") (OtherBodyIndex :type Integer) (bFromSweep :type Boolean) (SweepResult :type "HitResult Structure (by ref)"))
  (`|ExecutionSequence`
    (:`then_0`
      (bind _asbp_player (cast `/Game/InfiniteMatrix/Blueprints/BP_Player` OtherActor))
      (`/Game/InfiniteMatrix/Blueprints/BP_TunnelSpawner.SpawnTunnelAtSpawnPoint` (`self.TunnelSpawner`))
      (`self.K2_DestroyActor`)
      (if (`self.Collided`)
        (`/Game/InfiniteMatrix/Blueprints/BP_Player.ScoreUp` _asbp_player)
        (set `self.Collided` false)
        (`/Game/InfiniteMatrix/Blueprints/BP_Player.UpdateScoreUI` _asbp_player)
        (else
          (`/Game/InfiniteMatrix/Blueprints/BP_Player.ScoreUp` _asbp_player)
          (`GameplayStatics.PlaySoundAtLocation` "/Game/InfiniteMatrix/Audio/bonus-points-190035.bonus-points-190035" (`self.K2_GetActorLocation` _asbp_player) (struct) 1.0 1.0 0.0 null null null null)
          (`/Game/InfiniteMatrix/Blueprints/BP_Player.UpdateScoreUI` _asbp_player))))
    (:`then_1`
      (bind _asbp_projectile (cast `/Game/InfiniteMatrix/Blueprints/BP_Projectile` OtherActor))
      (`self.K2_DestroyActor` _asbp_projectile)
      (`KismetSystemLibrary.PrintString` "Projectile Destroyed"))))

(event `self.WallMesh.OnComponentBeginOverlap`
  (params (OverlappedComponent :type "PrimitiveComponent Object Reference") (OtherActor :type "Actor Object Reference") (OtherComp :type "PrimitiveComponent Object Reference") (OtherBodyIndex :type Integer) (bFromSweep :type Boolean) (SweepResult :type "HitResult Structure (by ref)"))
  (`KismetSystemLibrary.PrintString` "OnComponentBeginOverlap")
  (bind _asbp_player (cast `/Game/InfiniteMatrix/Blueprints/BP_Player` OtherActor))
  (if (> (`/Game/InfiniteMatrix/Blueprints/BP_Player.Health` _asbp_player) 0)
    (`/Game/InfiniteMatrix/Blueprints/BP_Player.HealthDown` _asbp_player)
    (`/Game/InfiniteMatrix/Blueprints/BP_Player.ScoreDown` _asbp_player)
    (set `self.Collided` true)
    (`/Game/InfiniteMatrix/Blueprints/BP_Player.UpdateHealthUI` _asbp_player)
    (`GameplayStatics.PlaySoundAtLocation` "/Game/InfiniteMatrix/Audio/thud-291047.thud-291047" (`self.K2_GetActorLocation` _asbp_player) (struct) 1.0 1.0 0.0 null null null null)
    (if (not (> (`/Game/InfiniteMatrix/Blueprints/BP_Player.Health` _asbp_player) 0))
      (set `/Game/InfiniteMatrix/Blueprints/BP_Player.IsDead` true _asbp_player)
      (`/Game/InfiniteMatrix/Blueprints/BP_Player.DisplayRestart` _asbp_player))))

(event `SpawnHealth`
  (bind _healthzone (`self.HealthZone`))
  (bind (_returnvalue_x _returnvalue_y _returnvalue_z) (`KismetMathLibrary.BreakVector` (`BoxComponent.GetScaledBoxExtent` _healthzone)))
  (bind (_returnvalue_x_2 _returnvalue_y_2 _returnvalue_z_2) (`KismetMathLibrary.BreakVector` (`SceneComponent.K2_GetComponentLocation` _healthzone)))
  (bind _asbp_player (cast `/Game/InfiniteMatrix/Blueprints/BP_Player` (`GameplayStatics.GetPlayerPawn` 0)))
  (if (< (`/Game/InfiniteMatrix/Blueprints/BP_Player.Health` _asbp_player) 15)
    (if (== (`KismetMathLibrary.RandomIntegerInRange` 0 4) 0)
      (bind _returnvalue (`|SpawnActorFromClass` "/Game/InfiniteMatrix/Blueprints/BP_Health.BP_Health_C" (`KismetMathLibrary.MakeTransform` (`KismetMathLibrary.MakeVector` (+ _returnvalue_x_2 (`KismetMathLibrary.RandomFloatInRange` (* _returnvalue_x -1.0) _returnvalue_x)) (+ _returnvalue_y_2 (`KismetMathLibrary.RandomFloatInRange` (* _returnvalue_y -1.0) _returnvalue_y)) (+ _returnvalue_z_2 (`KismetMathLibrary.RandomFloatInRange` (* _returnvalue_z -1.0) _returnvalue_z)))) "Undefined" "MultiplyWithRoot" null null))
      (`self.SetLifeSpan` _returnvalue 5.0))))

(event `SpawnEnemy`
  (bind _enemyzone (`self.EnemyZone`))
  (bind (_returnvalue_x _returnvalue_y _returnvalue_z) (`KismetMathLibrary.BreakVector` (`BoxComponent.GetScaledBoxExtent` _enemyzone)))
  (bind (_returnvalue_x_2 _returnvalue_y_2 _returnvalue_z_2) (`KismetMathLibrary.BreakVector` (`SceneComponent.K2_GetComponentLocation` _enemyzone)))
  (if (== (`KismetMathLibrary.RandomIntegerInRange` 0 3) 0)
    (bind _returnvalue (`|SpawnActorFromClass` "/Game/InfiniteMatrix/Blueprints/BP_Enemy.BP_Enemy_C" (`KismetMathLibrary.MakeTransform` (`KismetMathLibrary.MakeVector` (+ _returnvalue_x_2 (`KismetMathLibrary.RandomFloatInRange` 0.0 _returnvalue_x)) (+ _returnvalue_y_2 (`KismetMathLibrary.RandomFloatInRange` (* _returnvalue_y -1.0) _returnvalue_y)) (+ _returnvalue_z_2 (`KismetMathLibrary.RandomFloatInRange` (* _returnvalue_z -1.0) _returnvalue_z)))) "Undefined" "MultiplyWithRoot" null null))
    (`self.SetLifeSpan` _returnvalue 5.0)))

(fn `RandomizeWall`
  (`StaticMeshComponent.SetStaticMesh` (`self.WallMesh`) (select `int` (`KismetMathLibrary.RandomIntegerInRange` 0 3) :`0` "/Game/InfiniteMatrix/Meshes/SM_Hole_01.SM_Hole_01" :`1` "/Game/InfiniteMatrix/Meshes/SM_Hole_02.SM_Hole_02" :`2` "/Game/InfiniteMatrix/Meshes/SM_Hole_03.SM_Hole_03" :`3` "/Game/InfiniteMatrix/Meshes/SM_Hole_04.SM_Hole_04" :!type "StaticMesh Object Reference"))
  (`SceneComponent.K2_AddLocalRotation` (`self.WallMesh`) (`KismetMathLibrary.MakeRotator` (`KismetMathLibrary.RandomFloatInRange` 0.0 360.0)) false false))

(fn `UserConstructionScript`)